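; BP_50Bani is a coin pickup worth 50 for the Don't Fall game mode.
; A timeline, started from Tick, moves the Coin component vertically through its relative Z location.
; When the coin is hit by the third-person character, it adds 50 through GM_DontFall's AddCoin, plays a 2D sound and destroys itself.
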(event OnComponentHit(coin)
  (params (HitComponent :type Primitive%20Component%20Object%20Reference) (OtherActor :type Actor%20Object%20Reference) (OtherComp :type Primitive%20Component%20Object%20Reference) (NormalImpulse :type Vector :default "0, 0, 0") (Hit :type Hit%20Result%20Structure%20%28by%20ref%29))
  (Utilities|Casting|CastToBP_ThirdPersonCharacter OtherActor)
  (bind _asgm_dont_fall (Utilities|Casting|CastToGM_DontFall (Game|GetGameMode)))
  (Default|AddCoin _asgm_dont_fall 50)
  (Audio|PlaySound2D "/Game/Sounds/50bani.50bani" 1.0 1.0 0.0 0 0)
  (Actor|DestroyActor))

(event EventTick
  (params (DeltaSeconds :type Float%20%28single-precision%29))
  (bind _movement (Timeline|Timeline Play)
    (:Update
      (Transformation|SetRelativeLocation (Variables|Default|Getcoin) (Math|Vector|MakeVector 0.0 0.0 (* _movement 5e+01)) false false))))

(fn ConstructionScript)