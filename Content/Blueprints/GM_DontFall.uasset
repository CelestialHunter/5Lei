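; Game mode for a "Don't Fall" coin-collecting game, running the HUD, pause menu, restart key and end screens.
; AddCoin updates the coin total and HUD, while Tick checks for a player fall or a 500-coin win.
; P or Escape opens a menu without pausing the world, and R reopens Level1.
; ImpaleDeath shows its own end screen without setting GameOver, so Tick's checks stay active.
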(event Custom|AddCoin
  (params (Value :type Integer))
  ;[1 1 1] PickCoin
  (bind _output_get (Variables|Default|SetCoins (+ Value (Variables|Default|GetCoins))))
  (Default|UpdateBani (Variables|Default|GetUserInterface) _output_get))

(event Custom|Unpause
  ;[1 1 1] Unpause
  (Variables|Default|SetGamePaused false)
  (Widget|RemovefromParent (Variables|Default|GetescMenu))
  (Input|SetInputModeGameOnly (Game|GetPlayerController 0) false))

(event Custom|ImpaleDeath
  (bind _returnvalue (Game|GetPlayerController 0))
  (Audio|PlaySound2D "/Game/Sounds/spike.spike" 1.0 1.0 0.0 0 0)
  (Variables|Default|SetendMessage "Țeapă!")
  (bind _returnvalue_2 (UserInterface|CreateWidget "/Game/WBP_EndScreen.WBP_EndScreen_C"))
  (bind _aswbp_end_screen (Utilities|Casting|CastToWBP_EndScreen _returnvalue_2))
  (Variables|/Game/WBP_EndScreen.WBP_EndScreen_C|SetendMessageText _aswbp_end_screen (Variables|Default|GetendMessage))
  (UserInterface|Viewport|AddtoViewport _returnvalue_2 0)
  (Input|SetInputModeUIOnly _returnvalue _returnvalue_2 "DoNotLock" true)
  (Variables|/Script/Engine.PlayerController|SetbShowMouseCursor _returnvalue true))

(event EventTick
  (params (DeltaSeconds :type Float%20%28single-precision%29))
  (bind _returnvalue (Game|GetPlayerController 0))
  (bind _returnvalue_2 (Actor|GetActorOfClass "/Game/ThirdPerson/Blueprints/BP_ThirdPersonCharacter.BP_ThirdPersonCharacter_C"))
  (bind _output_get (Variables|Default|SetPlayer _returnvalue_2))
  (if (and (< (.z (Transformation|GetActorLocation _output_get)) -5.0) (not (Variables|Default|GetGameOver)))
    (Variables|Default|SetendMessage "Ai căzut!")
    (Audio|PlaySound2D "/Game/Sounds/wilhelmScream.wilhelmScream" 1.0 1.0 0.0 0 0)
    (Variables|Default|SetGameOver true :!label _label)
    (bind _returnvalue_3 (UserInterface|CreateWidget "/Game/WBP_EndScreen.WBP_EndScreen_C"))
    (bind _aswbp_end_screen (Utilities|Casting|CastToWBP_EndScreen _returnvalue_3))
    (Variables|/Game/WBP_EndScreen.WBP_EndScreen_C|SetendMessageText _aswbp_end_screen (Variables|Default|GetendMessage))
    (UserInterface|Viewport|AddtoViewport _returnvalue_3 0)
    (Input|SetInputModeUIOnly _returnvalue _returnvalue_3 "DoNotLock" true)
    (Variables|/Script/Engine.PlayerController|SetbShowMouseCursor _returnvalue true)
    (elif (and (>= (Variables|Default|GetCoins) 500) (not (Variables|Default|GetGameOver)))
      (Variables|Default|SetendMessage "Felicitări!")
      (Audio|PlaySound2D "/Game/Sounds/win.win" 1.0 1.0 0.0 0 0)
      (goto _label))))

(event EventBeginPlay
  (Input|EnableInput (Game|GetPlayerController 0))
  (bind _returnvalue (UserInterface|CreateWidget "/Game/WBP_UI.WBP_UI_C"))
  (bind _output_get (Variables|Default|SetUserInterface _returnvalue))
  (UserInterface|Viewport|AddtoViewport _output_get 0)
  (Input|SetInputModeGameOnly (Game|GetPlayerController 0) false))

(event Input|KeyboardEvents|Escape
  (params (Key :type Key%20Structure :default "None"))
  ;[1 1 1] Pause
  (:Pressed
    (if (not (Variables|Default|GetGamePaused))
      (Variables|Default|SetGamePaused true)
      (bind _returnvalue (UserInterface|CreateWidget "/Game/WBP_escMenu.WBP_escMenu_C"))
      (bind _output_get (Variables|Default|SetescMenu _returnvalue))
      (UserInterface|Viewport|AddtoViewport _output_get 0)
      (Input|SetInputModeUIOnly (Game|GetPlayerController 0) _output_get "DoNotLock" false))))

(event Input|KeyboardEvents|P
  (params (Key :type Key%20Structure :default "None"))
  ;[1 1 1] Pause
  (:Pressed
    (if (not (Variables|Default|GetGamePaused))
      (Variables|Default|SetGamePaused true)
      (bind _returnvalue (UserInterface|CreateWidget "/Game/WBP_escMenu.WBP_escMenu_C"))
      (bind _output_get (Variables|Default|SetescMenu _returnvalue))
      (UserInterface|Viewport|AddtoViewport _output_get 0)
      (Input|SetInputModeUIOnly (Game|GetPlayerController 0) _output_get "DoNotLock" false))))

(event Input|KeyboardEvents|R
  (params (Key :type Key%20Structure :default "None"))
  (:Pressed
    (Game|OpenLevel(byObjectReference) "/Game/Levels/Level1.Level1")))

(fn ConstructionScript)